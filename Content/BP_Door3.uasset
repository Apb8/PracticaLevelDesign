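; BP_Door3 is an automatic swinging door that opens while a BP_FirstPersonCharacter is inside its TriggerBox and closes when it leaves.
; Overlap begin and end set CanInteract and play or reverse the DoorTimer timeline, which scales Angle into the StaticMesh's relative yaw.
; Swing direction follows the player's side, estimated by comparing the normalized door-to-player vector to the door's forward vector with a loose 1.0 tolerance.
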(event OnComponentBeginOverlap(TriggerBox)
  (params (OverlappedComponent :type Primitive%20Component%20Object%20Reference) (OtherActor :type Actor%20Object%20Reference) (OtherComp :type Primitive%20Component%20Object%20Reference) (OtherBodyIndex :type Integer) (bFromSweep :type Boolean) (SweepResult :type Hit%20Result%20Structure%20%28by%20ref%29))
  (bind _asbp_first_person_character (Utilities|Casting|CastToBP_FirstPersonCharacter OtherActor))
  (Variables|Default|SetCanInteract true)
  (if true
    (Variables|Default|SetDirection (Utilities|Operators|EqualEqual (Math|Vector|Normalize (- (Transformation|GetActorLocation _asbp_first_person_character) (Transformation|GetActorLocation))) (Transformation|GetActorForwardVector) 1.0))
    (bind _doortimer (Timeline|DoorTimer Play)
      (:Update
        (Transformation|SetRelativeRotation (Variables|Default|GetStaticMesh) (Math|Rotator|MakeRotator 0.0 0.0 (* _doortimer (Variables|Default|GetAngle) (Math|Float|SelectFloat 1.0 -1.0 (Variables|Default|GetDirection)))) false false)))))

(event OnComponentEndOverlap(TriggerBox)
  (params (OverlappedComponent :type Primitive%20Component%20Object%20Reference) (OtherActor :type Actor%20Object%20Reference) (OtherComp :type Primitive%20Component%20Object%20Reference) (OtherBodyIndex :type Integer))
  (Utilities|Casting|CastToBP_FirstPersonCharacter OtherActor)
  (Variables|Default|SetCanInteract false)
  (bind _doortimer (Timeline|DoorTimer Reverse)
    (:Update
      (Transformation|SetRelativeRotation (Variables|Default|GetStaticMesh) (Math|Rotator|MakeRotator 0.0 0.0 (* _doortimer (Variables|Default|GetAngle) (Math|Float|SelectFloat 1.0 -1.0 (Variables|Default|GetDirection)))) false false))))

(event EventBeginPlay)

(event Collision|EventActorBeginOverlap
  (params (OtherActor :type Actor%20Object%20Reference)))

(event EventTick
  (params (DeltaSeconds :type Float%20%28single-precision%29)))

(fn ConstructionScript)